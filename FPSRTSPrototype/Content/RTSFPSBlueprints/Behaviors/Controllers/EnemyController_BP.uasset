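; Enemy AI controller that turns PawnSensing sight and hearing events into Blackboard entries.
; Seen pawns are stored as AllyActor only if they cast to AllyMember and then AllyForGeneral_01.
; Noises closer to the controlled pawn than HearingDistance set LocationOfSound and raise HasHeardSound.
; This graph only writes these keys; it neither clears them nor starts a behavior tree.
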(event OnHearNoise(PawnSensing)
  (params (Instigator :type Pawn%20Object%20Reference) (Location :type Vector%20%28by%20ref%29) (Volume :type Float%20%28single-precision%29))
  (bind _self self)
  (bind _blackboard (Variables|Default|GetBlackboard _self))
  (if (< (Math|Vector|VectorLength (- Location (Pawn|GetNavAgentLocation (Pawn|GetControlledPawn)))) (Variables|Default|GetHearingDistance))
    (AI|Components|Blackboard|SetValueasVector _blackboard (Utilities|Name|MakeLiteralName "LocationOfSound") Location)
    (AI|Components|Blackboard|SetValueasBool _blackboard (Utilities|Name|MakeLiteralName "HasHeardSound") true)))

(event OnSeePawn(PawnSensing)
  (params (Pawn :type Pawn%20Object%20Reference))
  (bind _asally_member (Utilities|Casting|CastToAllyMember Pawn))
  (bind _asally_for_general_01 (Utilities|Casting|CastToAllyForGeneral_01 _asally_member))
  (AI|Components|Blackboard|SetValueasObject (Variables|Default|GetBlackboard self) (Utilities|Name|MakeLiteralName "AllyActor") _asally_for_general_01))

(event EventBeginPlay)

(fn ConstructionScript)