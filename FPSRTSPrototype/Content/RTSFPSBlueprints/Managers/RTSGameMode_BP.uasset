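; RTS game mode that sets up the player's spectator and UI when play begins.
; BeginPlay calls SpawnMainSpectator, then creates the RTSPlayerUI widget and adds it to the viewport.
; SpawnMainSpectator takes the first spectator subclass, casts it to Spectator_01_BP and spawns it at the game mode's root transform.
; An empty Spectators array prints a warning instead of spawning.
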(event EventBeginPlay
  (CallFunction|SpawnMainSpectator)
  (bind _returnvalue (UserInterface|CreateWidget "/Game/RTSFPSBlueprints/UI/RTSPlayerUI.RTSPlayerUI_C"))
  (UserInterface|Viewport|AddtoViewport _returnvalue 0))

(event EventTick
  (params (DeltaSeconds :type Float%20%28single-precision%29)))

(fn ConstructionScript)

(fn SpawnMainSpectator
  (if (> (Utilities|Array|Length (Variables|Default|GetSpectators)) 0)
    (bind _returnvalue (Class|RTSProtoGameMode|GetSpectatorSubClass))
    (bind _asspectator_01_bp (Utilities|Casting|CastToSpectator_01_BPClass _returnvalue))
    (Game|SpawnActorfromClass _asspectator_01_bp (Transformation|GetWorldTransform (Variables|Default|GetDefaultSceneRoot self)) "Undefined" 0 0)
    (else
      (Development|PrintString "There is no Spectator in GameMode Array!!!!!!!"))))